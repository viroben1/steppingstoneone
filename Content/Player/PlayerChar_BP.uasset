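; PlayerChar_BP is the player character Blueprint that sets up the on-screen UI and toggles a crafting menu.
; On BeginPlay it creates and stores the player and objective widgets and adds both to the viewport.
; The CraftMenu input runs a FlipFlop that either creates a fresh crafting widget with mouse cursor and Game and UI input, or removes it and restores game-only input and viewport focus.
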(event `self.ReceiveBeginPlay`
  (bind _returnvalue (`|CreateWidget` "/Game/Widgets/Player_W.Player_W_C" (`GameplayStatics.GetPlayerController` 0)))
  (bind _output_get (set `self.playerUI` _returnvalue))
  (`UserWidget.AddToViewport` _output_get 0)
  (bind _returnvalue_2 (`|CreateWidget` "/Game/Widgets/Objective_W.Objective_W_C" (`GameplayStatics.GetPlayerController` 0)))
  (bind _output_get_2 (set `self.objWidget` _returnvalue_2))
  (`UserWidget.AddToViewport` _output_get_2 0))

(event `InputAction|CraftMenu`
  (params (Key :type "Key Structure"))
  (bind _returnvalue (`GameplayStatics.GetPlayerController` 0))
  (:`Pressed`
    (`/Engine/EditorBlueprintResources/StandardMacros.FlipFlop`
      (:`A`
        (bind _returnvalue_2 (`|CreateWidget` "/Game/Widgets/Crafting_W.Crafting_W_C" (`GameplayStatics.GetPlayerController` 0)))
        (`UserWidget.AddToViewport` _returnvalue_2 0)
        (set `PlayerController.bShowMouseCursor` true _returnvalue)
        (`WidgetBlueprintLibrary.SetInputMode_GameAndUIEx` _returnvalue _returnvalue_2))
      (:`B`
        (`Widget.RemoveFromParent` _returnvalue_2)
        (set `PlayerController.bShowMouseCursor` false _returnvalue)
        (`WidgetBlueprintLibrary.SetInputMode_GameOnly` _returnvalue)
        (`WidgetBlueprintLibrary.SetFocusToGameViewport`)))))

(fn `UserConstructionScript`)